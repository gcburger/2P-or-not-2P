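; BP_MovingCollision is an actor for moving objects such as platforms, with separately set visual and collision meshes, the collision mesh offset by a relative transform.
; Its move functions save the prior location for resetting, optionally sweep, and report blocking hits filtered through an ignored-class list.
; An attach function parents other actors, such as buttons, and sets move-ignore on them and their child actors so movement does not get stuck.
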(event Collision|EventActorBeginOverlap
  (params (OtherActor :type Actor%20Object%20Reference)))

(event EventTick
  (params (DeltaSeconds :type Float%20%28single-precision%29)))

(fn ConstructionScript
  (bind _visualmesh (Variables|Default|GetVisualMesh))
  (bind _collisionmesh (Variables|Default|GetCollisionMesh))
  (bind _collision (Variables|Default|GetCollision))
  ;[1 1 1] Set the mesh for the visual and collision component separately, and offset the colliison by the desired amount.
  (Utilities|IsValid _visualmesh
    (:Is%20Valid
      (Components|StaticMesh|SetStaticMesh (Variables|Default|GetVisual) _visualmesh))
    (:Is%20Not%20Valid
      _))
  (Utilities|IsValid _collisionmesh
    (:Is%20Valid
      (Components|StaticMesh|SetStaticMesh _collision _collisionmesh)
      (Transformation|SetRelativeTransform _collision (Variables|Default|GetSurroundingMeshRelativeTransform) false false))))

(fn MCAddLocalOffset
  (params (Offset :type Vector) (SweepCollision :type Boolean))
  ;[1 1 1] Add local offset to actor, and returns whether the resulting movement collided with another actor.
  ; Stores the location PRIOR to moving, in case it needs to reset to that location as a result of colliding.
  (Variables|INTERNAL_LOGIC|SetLocationBeforeMoving (Transformation|GetActorLocation))
  (bind _sweephitresult (Transformation|AddActorLocalOffset Offset SweepCollision false))
  (bind _output_get (Variables|INTERNAL_LOGIC|SetIsBlocked (and (.bBlockingHit (Collision|BreakHitResult _sweephitresult)) (CallFunction|IsValidCollisionActor (.HitActor (Collision|BreakHitResult _sweephitresult))))))
  (return _output_get))

(fn MCSetRelativeLocation
  (params (Location :type Vector) (SweepCollision :type Boolean))
  ;[1 1 1] Set the relative location of this actor, and returns whether the resulting movement collided with another actor.
  ; Stores the location PRIOR to moving, in case it needs to reset to that location as a result of colliding.
  (Variables|INTERNAL_LOGIC|SetLocationBeforeMoving (Transformation|GetActorLocation))
  (bind _sweephitresult (Transformation|SetActorRelativeLocation Location SweepCollision))
  (bind _output_get (Variables|INTERNAL_LOGIC|SetIsBlocked (and (.bBlockingHit (Collision|BreakHitResult _sweephitresult)) (CallFunction|IsValidCollisionActor (.HitActor (Collision|BreakHitResult _sweephitresult))))))
  (return _output_get))

(fn MCResettoPreviousLocation
  ;[1 1 1] Reset actor to previous location before it was moved.
  (Transformation|SetActorLocation (Variables|INTERNAL_LOGIC|GetLocationBeforeMoving) false false))

(fn MCSetWorldLocation
  (params (Location :type Vector) (SweepCollision :type Boolean))
  ;[1 1 1] Set's the world location of the actor, and returns whether the resulting movement collided with another actor.
  ; Stores the location PRIOR to moving, in case it needs to reset to that location as a result of colliding.
  (Variables|INTERNAL_LOGIC|SetLocationBeforeMoving (Transformation|GetActorLocation))
  (bind _sweephitresult (Transformation|SetActorLocation Location SweepCollision false))
  (bind _output_get (Variables|INTERNAL_LOGIC|SetIsBlocked (and (.bBlockingHit (Collision|BreakHitResult _sweephitresult)) (CallFunction|IsValidCollisionActor (.HitActor (Collision|BreakHitResult _sweephitresult))))))
  (return _output_get))

(fn AttachActorsandIgnoreCollision
  (params (Actors :type Array%20of%20Actor%20Object%20References))
  (bind _visual (Variables|Default|GetVisual))
  ;[1 1 1] Attaches another actor to this actor. For example attaching a button to a moving platform.
  ; Also set this moving collision actor to ignore the child actor when moving, otherwise it will get "stuck every time it moves".
  (bind _output_get (LocalVariables|SetTempChildActors Actors))
  (for _array_element _output_get
    (if (!= _array_element self)
      (Transformation|AttachActorToActor _array_element self "None" "KeepRelative" "KeepRelative" "KeepRelative" true)
      (Collision|IgnoreActorwhenMoving _visual _array_element true)
      (for _array_element_2 (Actor|GetAllChildActors _array_element true)
        (Collision|IgnoreActorwhenMoving _visual _array_element_2 true)
        (bind _asbp_moving_collision (Utilities|Casting|CastToBP_MovingCollision _array_element_2))
        (Collision|IgnoreActorwhenMoving (Variables|BP_MovingCollision_C|GetVisual _asbp_moving_collision) self true)))))

(fn IsValidCollisionActor
  (params (Actor :type Actor%20Object%20Reference))
  (bind _returnvalue (Utilities|GetClass Actor))
  (bind _actorstoignore (Variables|Default|GetActorsToIgnore))
  ;[1 1 1] Checks if the actor is of a class that should be ignored.
  (bind _array_element (Utilities|Array|ForEachLoopwithBreak _actorstoignore :!label _label)
    (:LoopBody
      (if (Utilities|ClassIsChildOf _returnvalue _array_element)
        (LocalVariables|SetValid false)
        (goto _label Break)))
    (:Completed
      (if (Utilities|Array|ContainsItem _actorstoignore _returnvalue)
        (LocalVariables|SetValid false))
      (return (LocalVariables|GetValid)))))